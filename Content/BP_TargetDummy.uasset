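; BP_TargetDummy is a target dummy actor that loses health when hit and destroys itself at zero.
; Its Takehit function subtracts a fixed amount from Health, prints the new value and destroys the actor once Health is depleted.
; BeginPlay prints the starting Health, while the overlap, Tick and construction script do nothing, so damage depends on Takehit being called.
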(event EventBeginPlay
  (Development|PrintString (Utilities|String|ToString(Float) (Variables|Default|Gethealth))))

(event Collision|EventActorBeginOverlap
  (params (OtherActor :type Actor%20Object%20Reference)))

(event EventTick
  (params (DeltaSeconds :type Float%20%28single-precision%29)))

(fn ConstructionScript)

(fn Takehit
  (Variables|Default|Sethealth (- (Variables|Default|Gethealth) 25.0))
  (Development|PrintString (Utilities|String|ToString(Float) (Variables|Default|Gethealth)))
  (if (<= (Variables|Default|Gethealth) 0.0)
    (Actor|DestroyActor)))